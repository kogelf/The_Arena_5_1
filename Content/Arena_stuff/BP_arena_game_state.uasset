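; Arena game state that tracks the player list, player count and full-death count, and shows the win screen.
; update_player_list copies PlayerArray into AddPlayerStates, whose OnRep refreshes every Kills_counter_BP widget for the kill display.
; fulldeadadd increments the death total, and End_game creates You_win_screen_BP for the given player.
; Fulldead is empty, and the logic to find surviving winners and show the cursor is disconnected.
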(event `update_player_list`
  ;[1 1 1] updates player list for kill count
  (set `self.add Player states` (`self.PlayerArray`))
  (set `self.Players` (+ (`self.Players`) 1))
  (`KismetArrayLibrary.Array_Add` (`self.All players`)))

(event `Full dead`)

(event `full dead add`
  (set `self.All_full_deaths` (+ (`self.All_full_deaths`) 1)))

(event `End_game`
  (params (Target :type "PlayerController Object Reference"))
  (bind _returnvalue (`|CreateWidget` "/Game/Arena_stuff/charecture_folder/universal_hud_folder/END_screen_folder/you_win_screen_BP.you_win_screen_BP_C" Target))
  (`UserWidget.AddToViewport` _returnvalue 0))

(fn `OnRep_add Player states`
  (bind _foundwidgets (`WidgetBlueprintLibrary.GetAllWidgetsOfClass` "/Game/Arena_stuff/charecture_folder/universal_hud_folder/kills_counter_BP.kills_counter_BP_C" false))
  (for _array_element _foundwidgets
    (`/Game/Arena_stuff/charecture_folder/universal_hud_folder/kills_counter_BP.event update list` _array_element)))

(fn `OnRep_Player Array`)

(fn `UserConstructionScript`)