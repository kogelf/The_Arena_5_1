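; GK-22 projectile Blueprint that damages and knocks back whatever it strikes.
; When its Sphere3 component hits an actor other than its owner, it applies fixed damage credited to the instigator's controller and owner.
; It then sends a KnockbackMessage to the hit actor along the sphere's forward vector and destroys itself.
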(event `self.Sphere3.OnComponentHit`
  (params (HitComponent :type "PrimitiveComponent Object Reference") (OtherActor :type "Actor Object Reference") (OtherComp :type "PrimitiveComponent Object Reference") (NormalImpulse :type "Vector Structure") (Hit :type "HitResult Structure (by ref)"))
  (bind (_bblockinghit _binitialoverlap _time _distance _location _impactpoint _normal _impactnormal _physmat _hitactor) (`GameplayStatics.BreakHitResult` Hit))
  (bind _returnvalue (`self.GetOwner`))
  (if (not (== OtherActor _returnvalue))
    (`GameplayStatics.ApplyDamage` _hitactor 20.0 (`self.GetInstigatorController`) _returnvalue)
    (message `/Game/Arena_stuff/status_efects/status_efects_interface.knockback` _hitactor 100.0 (`SceneComponent.GetForwardVector` (`self.Sphere3`)))
    (`self.K2_DestroyActor`)))

(fn `UserConstructionScript`
  (`parent.UserConstructionScript`))