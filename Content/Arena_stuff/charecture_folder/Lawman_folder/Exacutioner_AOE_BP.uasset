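; Area-of-effect actor for the Lawman's Executioner that damages and knocks back actors entering its sphere.
; Each overlap runs a debug-drawn Visibility trace from the particle system's location to the actor, so blocking geometry can intercept the effect.
; The hit actor, if damageable, receives a knockback message, with the impact location passed as its forward vector, and fixed damage credited to the first player controller.
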(event `self.Sphere.OnComponentBeginOverlap`
  (params (OverlappedComponent :type "PrimitiveComponent Object Reference") (OtherActor :type "Actor Object Reference") (OtherComp :type "PrimitiveComponent Object Reference") (OtherBodyIndex :type Integer) (bFromSweep :type Boolean) (SweepResult :type "HitResult Structure (by ref)"))
  (bind _returnvalue (`GameplayStatics.GetPlayerController` 0))
  (for _array_element (`|MakeArray` OtherActor)
    (bind (_outhit _returnvalue_2) (`KismetSystemLibrary.LineTraceSingle` :`Start` (`SceneComponent.K2_GetComponentLocation` (`self.ParticleSystem`)) :`End` (`self.K2_GetActorLocation` _array_element) :`TraceChannel` "TraceTypeQuery1" :`DrawDebugType` "ForDuration"))
    (if _returnvalue_2
      (bind (_bblockinghit _binitialoverlap _time _distance _location _impactpoint _normal _impactnormal _physmat _hitactor) (`GameplayStatics.BreakHitResult` _outhit))
      (if (`Actor.bCanBeDamaged` _hitactor)
        (message `/Game/Arena_stuff/status_efects/status_efects_interface.knockback` _hitactor 300.0 _location)
        (`GameplayStatics.ApplyDamage` _hitactor 10.0 _returnvalue _returnvalue)))))

(fn `UserConstructionScript`)