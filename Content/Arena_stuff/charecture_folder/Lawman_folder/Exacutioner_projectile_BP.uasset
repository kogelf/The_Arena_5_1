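; Projectile actor for the Lawman's Executioner attack that damages and knocks back what it hits, then leaves an area-of-effect actor.
; A sphere hit on anything but its owner applies damage credited to player controller 0, sends a knockback message using the impact point as ForwardVector, and destroys the projectile.
; On Destroyed, whatever the cause, it spawns Exacutioner_AOE_BP at the sphere's location, with its Instigator as owner and instigator.
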(event `self.Sphere3.OnComponentHit`
  (params (HitComponent :type "PrimitiveComponent Object Reference") (OtherActor :type "Actor Object Reference") (OtherComp :type "PrimitiveComponent Object Reference") (NormalImpulse :type "Vector Structure") (Hit :type "HitResult Structure (by ref)"))
  (bind (_bblockinghit _binitialoverlap _time _distance _location _impactpoint _normal _impactnormal _physmat _hitactor) (`GameplayStatics.BreakHitResult` Hit))
  (bind _returnvalue (`self.GetOwner`))
  (if (not (== OtherActor _returnvalue))
    (`GameplayStatics.ApplyDamage` _hitactor 20.0 (`GameplayStatics.GetPlayerController` 0) _returnvalue)
    (message `/Game/Arena_stuff/status_efects/status_efects_interface.knockback` _hitactor 250.0 _impactpoint)
    (`self.K2_DestroyActor`)))

(event `self.ReceiveDestroyed`
  (bind _instigator (`self.Instigator`))
  (`self.spawn bomb` _instigator _instigator (`KismetMathLibrary.Conv_VectorToTransform` (`SceneComponent.K2_GetComponentLocation` (`self.Sphere3`)))))

(event `spawn bomb`
  (params (Owner :type "Actor Object Reference") (Instigator :type "Pawn Object Reference") (SpawnTransform :type "Transform Structure"))
  (`|SpawnActorFromClass` "/Game/Arena_stuff/charecture_folder/Lawman_folder/Exacutioner_AOE_BP.Exacutioner_AOE_BP_C" SpawnTransform "AlwaysSpawn" "OverrideRootScale" Owner Instigator))

(fn `UserConstructionScript`
  (`parent.UserConstructionScript`))