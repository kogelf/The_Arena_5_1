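; Projectile actor for the Lawman character's tazer that damages and debuffs whatever it hits.
; When its sphere component hits an actor other than its owner, it applies damage, credited to the owner and instigated by player controller 0.
; It then sends the hit actor knockback, smoked, slowness and weakness messages, passing the impact point as the knockback's forward vector.
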(event `self.Sphere3.OnComponentHit`
  (params (HitComponent :type "PrimitiveComponent Object Reference") (OtherActor :type "Actor Object Reference") (OtherComp :type "PrimitiveComponent Object Reference") (NormalImpulse :type "Vector Structure") (Hit :type "HitResult Structure (by ref)"))
  (bind (_bblockinghit _binitialoverlap _time _distance _location _impactpoint _normal _impactnormal _physmat _hitactor) (`GameplayStatics.BreakHitResult` Hit))
  (bind _returnvalue (`self.GetOwner`))
  (if (not (== OtherActor _returnvalue))
    (`GameplayStatics.ApplyDamage` _hitactor 30.0 (`GameplayStatics.GetPlayerController` 0) _returnvalue)
    (message `/Game/Arena_stuff/status_efects/status_efects_interface.knockback` _hitactor 250.0 _impactpoint)
    (message `/Game/Arena_stuff/status_efects/status_efects_interface.Smoked` _hitactor 2.0)
    (message `/Game/Arena_stuff/status_efects/status_efects_interface.slownes` _hitactor 2.0 1000.0)
    (message `/Game/Arena_stuff/status_efects/status_efects_interface.weeknes` _hitactor 2.0 100.0)))

(fn `UserConstructionScript`
  (`parent.UserConstructionScript`))