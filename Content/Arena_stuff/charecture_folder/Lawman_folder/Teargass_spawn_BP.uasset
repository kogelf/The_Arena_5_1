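; Teargass_spawn_BP is the Lawman's tear gas carrier actor, which leaves a gas area where it is destroyed.
; A hit on its Sphere3 component by any actor other than its owner destroys it.
; The Destroyed event then calls a spawn event that creates Teargass_Aoe_BP at the sphere's world location, regardless of collisions.
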(event `self.Sphere3.OnComponentHit`
  (params (HitComponent :type "PrimitiveComponent Object Reference") (OtherActor :type "Actor Object Reference") (OtherComp :type "PrimitiveComponent Object Reference") (NormalImpulse :type "Vector Structure") (Hit :type "HitResult Structure (by ref)"))
  (if (not (== OtherActor (`self.GetOwner`)))
    (`self.K2_DestroyActor`)))

(event `self.ReceiveDestroyed`
  (`self.spawn gass`))

(event `spawn gass`
  (`|SpawnActorFromClass` "/Game/Arena_stuff/charecture_folder/Lawman_folder/teargass_Aoe_BP.teargass_Aoe_BP_C" (`KismetMathLibrary.Conv_VectorToTransform` (`SceneComponent.K2_GetComponentLocation` (`self.Sphere3`))) "AlwaysSpawn" "OverrideRootScale" null null))

(fn `UserConstructionScript`
  (`parent.UserConstructionScript`))