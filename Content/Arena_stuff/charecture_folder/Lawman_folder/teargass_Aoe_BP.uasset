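; Lawman tear gas area-of-effect actor that poisons and slows damageable actors entering its sphere.
; On sphere begin overlap, it line traces on the Visibility channel from the particle system to the overlapping actor's location.
; The first actor the trace hits, which may differ from the overlapping one, receives timed poison and slowness messages if it can be damaged.
; Effects are sent only on overlap begin, with no periodic reapplication.
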(event `self.Sphere.OnComponentBeginOverlap`
  (params (OverlappedComponent :type "PrimitiveComponent Object Reference") (OtherActor :type "Actor Object Reference") (OtherComp :type "PrimitiveComponent Object Reference") (OtherBodyIndex :type Integer) (bFromSweep :type Boolean) (SweepResult :type "HitResult Structure (by ref)"))
  (for _array_element (`|MakeArray` OtherActor)
    (bind (_outhit _returnvalue) (`KismetSystemLibrary.LineTraceSingle` (`SceneComponent.K2_GetComponentLocation` (`self.ParticleSystem`)) (`self.K2_GetActorLocation` _array_element) "TraceTypeQuery1"))
    (if _returnvalue
      (bind (_bblockinghit _binitialoverlap _time _distance _location _impactpoint _normal _impactnormal _physmat _hitactor) (`GameplayStatics.BreakHitResult` _outhit))
      (if (`Actor.bCanBeDamaged` _hitactor)
        (message `/Game/Arena_stuff/status_efects/status_efects_interface.poision` _hitactor 7.0 4)
        (message `/Game/Arena_stuff/status_efects/status_efects_interface.slownes` _hitactor 7.0 50.0)))))

(fn `UserConstructionScript`)