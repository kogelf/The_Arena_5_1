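; Weaver's grappling hook projectile that reels its owning BP_FirstPersonCharacter toward the point where it hits.
; On component hit it stores the grab point on the owner, switches movement to Flying and shows the cable.
; While grappling, Tick updates the cable end and applies a constant-strength force toward that point, skewed sideways by right/left input.
; Destroying the projectile clears the grapple, hides the cable and returns the owner to Falling.
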(event `self.ReceiveTick`
  (params (DeltaSeconds :type "Float (single-precision)"))
  (bind _asbp_first_person_character (cast `/Game/Arena_stuff/BP_FirstPersonCharacter` (`self.GetOwner`)))
  (if (`/Game/Arena_stuff/BP_FirstPersonCharacter.is grappling ` _asbp_first_person_character)
    (set `CableComponent.EndLocation` (`KismetMathLibrary.InverseTransformLocation` (`self.GetTransform` _asbp_first_person_character) (`/Game/Arena_stuff/BP_FirstPersonCharacter.grab point` _asbp_first_person_character)) (`/Game/Arena_stuff/BP_FirstPersonCharacter.Cable` _asbp_first_person_character))
    (`CharacterMovementComponent.AddForce` (`Character.CharacterMovement` _asbp_first_person_character) (* (`KismetMathLibrary.Normal` (+ (`KismetMathLibrary.GetDirectionUnitVector` (`self.K2_GetActorLocation` _asbp_first_person_character) (`/Game/Arena_stuff/BP_FirstPersonCharacter.grab point` _asbp_first_person_character)) (* (* (`self.GetActorRightVector` _asbp_first_person_character) (`self.GetInputAxisValue`)) 0.7))) 250000.0))))

(event `self.Sphere2.OnComponentHit`
  (params (HitComponent :type "PrimitiveComponent Object Reference") (OtherActor :type "Actor Object Reference") (OtherComp :type "PrimitiveComponent Object Reference") (NormalImpulse :type "Vector Structure") (Hit :type "HitResult Structure (by ref)"))
  (bind _asbp_first_person_character (cast `/Game/Arena_stuff/BP_FirstPersonCharacter` (`self.GetOwner`)))
  (set `/Game/Arena_stuff/BP_FirstPersonCharacter.grab point` (`SceneComponent.K2_GetComponentLocation` (`self.Sphere3`)) _asbp_first_person_character)
  (set `/Game/Arena_stuff/BP_FirstPersonCharacter.is grappling ` true _asbp_first_person_character)
  (`CharacterMovementComponent.SetMovementMode` (`Character.CharacterMovement` _asbp_first_person_character) "MOVE_Flying" 0)
  (`SceneComponent.SetVisibility` (`/Game/Arena_stuff/BP_FirstPersonCharacter.Cable` _asbp_first_person_character) true false))

(event `self.ReceiveDestroyed`
  (bind _asbp_first_person_character (cast `/Game/Arena_stuff/BP_FirstPersonCharacter` (`self.GetOwner`)))
  (set `/Game/Arena_stuff/BP_FirstPersonCharacter.is grappling ` false _asbp_first_person_character)
  (set `/Game/Arena_stuff/BP_FirstPersonCharacter.grab point` (0.0 0.0 0.0) _asbp_first_person_character)
  (`SceneComponent.SetVisibility` (`/Game/Arena_stuff/BP_FirstPersonCharacter.Cable` _asbp_first_person_character) false false)
  (`CharacterMovementComponent.SetMovementMode` (`Character.CharacterMovement` _asbp_first_person_character) "MOVE_Falling" 0))

(fn `UserConstructionScript`
  (`parent.UserConstructionScript`))