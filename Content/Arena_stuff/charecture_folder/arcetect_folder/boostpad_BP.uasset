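; Boost pad actor that launches the first-person character and grants timed status effects on contact.
; On box overlap, a StatusServer event sends speed and ward messages to the overlapping actor, before any character check.
; If that actor is a BP_FirstPersonCharacter, it is then launched along the pad root's forward vector at a fixed speed, added to its current velocity rather than overriding it.
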(event `self.Box.OnComponentBeginOverlap`
  (params (OverlappedComponent :type "PrimitiveComponent Object Reference") (OtherActor :type "Actor Object Reference") (OtherComp :type "PrimitiveComponent Object Reference") (OtherBodyIndex :type Integer) (bFromSweep :type Boolean) (SweepResult :type "HitResult Structure (by ref)"))
  (`self.status server` OtherActor)
  (bind _asbp_first_person_character (cast `/Game/Arena_stuff/BP_FirstPersonCharacter` OtherActor))
  (`Character.LaunchCharacter` _asbp_first_person_character (* (`SceneComponent.GetForwardVector` (`self.DefaultSceneRoot`)) 2000.0) false false))

(event `status server`
  (params (Target :type "Object Object Reference"))
  (message `/Game/Arena_stuff/status_efects/status_efects_interface.speed` Target 10.0 50.0)
  (message `/Game/Arena_stuff/status_efects/status_efects_interface.ward` Target 10.0 50.0))

(fn `UserConstructionScript`)