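; Headhunter trap spawner actor, which turns into a Head_hunter_trap_BP where it hits something.
; When its Sphere3 component registers a hit, it spawns the trap at the sphere's location, always spawning regardless of collision, then destroys itself.
; The trap's rotation comes from the sphere's forward vector flattened to 2D, keeping only its yaw so the trap stands level.
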(event `self.Sphere3.OnComponentHit`
  (params (HitComponent :type "PrimitiveComponent Object Reference") (OtherActor :type "Actor Object Reference") (OtherComp :type "PrimitiveComponent Object Reference") (NormalImpulse :type "Vector Structure") (Hit :type "HitResult Structure (by ref)"))
  (bind _sphere3 (`self.Sphere3`))
  (`|SpawnActorFromClass` "/Game/Arena_stuff/charecture_folder/headhunter_folder/head_hunter_trap_BP.head_hunter_trap_BP_C" (`KismetMathLibrary.MakeTransform` (`SceneComponent.K2_GetComponentLocation` _sphere3) (`KismetMathLibrary.Conv_VectorToRotator` (`KismetMathLibrary.Vector_Normal2D` (`KismetMathLibrary.Conv_RotatorToVector` (`SceneComponent.K2_GetComponentRotation` _sphere3))))) "AlwaysSpawn" "OverrideRootScale" null null)
  (`self.K2_DestroyActor`))

(fn `UserConstructionScript`
  (`parent.UserConstructionScript`))