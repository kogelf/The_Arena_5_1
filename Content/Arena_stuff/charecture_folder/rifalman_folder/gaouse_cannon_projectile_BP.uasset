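; Gauss cannon projectile, filed under the rifleman character, that damages what it strikes and attempts follow-through damage behind it.
; A hit on its sphere component deals heavy damage to the struck actor, then runs a short forward multi box trace on Visibility with debug drawing.
; Each trace hit takes half that damage.
; The projectile destroys itself inside that loop, so it survives an impact when the trace finds nothing.
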(event `self.Sphere3.OnComponentHit`
  (params (HitComponent :type "PrimitiveComponent Object Reference") (OtherActor :type "Actor Object Reference") (OtherComp :type "PrimitiveComponent Object Reference") (NormalImpulse :type "Vector Structure") (Hit :type "HitResult Structure (by ref)"))
  (bind _sphere3 (`self.Sphere3`))
  (bind _returnvalue (`SceneComponent.K2_GetComponentLocation` _sphere3))
  (`GameplayStatics.ApplyDamage` OtherActor 100.0)
  (bind _outhits (`KismetSystemLibrary.BoxTraceMulti` :`Start` _returnvalue :`End` (+ (* (`SceneComponent.GetForwardVector` _sphere3) 200.0) _returnvalue) :`HalfSize` (3.0 3.0 3.0) :`TraceChannel` "TraceTypeQuery1" :`DrawDebugType` "ForDuration"))
  (for _array_element _outhits
    (`GameplayStatics.ApplyDamage` (`.HitActor` (`GameplayStatics.BreakHitResult` _array_element)) 50.0)
    (`self.K2_DestroyActor`)))

(fn `UserConstructionScript`
  (`parent.UserConstructionScript`))