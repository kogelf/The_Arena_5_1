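; Explosion actor for the rifleman that applies damage and knockback when actors overlap its sphere.
; Each overlap runs a debug-drawn Visibility trace from the root to the overlapping actor, so whatever blocks it first becomes the hit.
; On a hit it calls ApplyDamage with no damaged actor shown, then sends KnockbackMessage to the hit actor, passing the impact point as the forward vector.
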(event `self.Sphere.OnComponentBeginOverlap`
  (params (OverlappedComponent :type "PrimitiveComponent Object Reference") (OtherActor :type "Actor Object Reference") (OtherComp :type "PrimitiveComponent Object Reference") (OtherBodyIndex :type Integer) (bFromSweep :type Boolean) (SweepResult :type "HitResult Structure (by ref)"))
  (for _ (`|MakeArray` OtherActor)
    (bind (_outhit _returnvalue) (`KismetSystemLibrary.LineTraceSingle` :`Start` (`SceneComponent.K2_GetComponentLocation` (`self.DefaultSceneRoot`)) :`End` (`self.K2_GetActorLocation` OtherActor) :`TraceChannel` "TraceTypeQuery1" :`DrawDebugType` "ForDuration"))
    (if _returnvalue
      (bind (_bblockinghit _binitialoverlap _time _distance _location _impactpoint _normal _impactnormal _physmat _hitactor) (`GameplayStatics.BreakHitResult` _outhit))
      (set `self.Hit Actor` _hitactor)
      (`GameplayStatics.ApplyDamage` null 50.0)
      (message `/Game/Arena_stuff/status_efects/status_efects_interface.knockback` _hitactor 4000.0 _impactpoint))))

(fn `UserConstructionScript`)