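; Rifleman grenade actor that leaves an explosion behind when it is destroyed.
; On Destroyed it spawns an enlarged Rifalman_exsplosio_BP at the Sphere3 component's world location, regardless of collision.
; The explosion faces along the sphere's forward vector flattened to the horizontal plane.
; BeginPlay, overlap and Tick are disabled stubs, so the graph holds no movement, fuse or impact logic.
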(event `self.ReceiveDestroyed`
  (bind _sphere3 (`self.Sphere3`))
  (`|SpawnActorFromClass` "/Game/Arena_stuff/charecture_folder/rifalman_folder/rifalman_exsplosio_BP.rifalman_exsplosio_BP_C" (`KismetMathLibrary.MakeTransform` (`SceneComponent.K2_GetComponentLocation` _sphere3) (`KismetMathLibrary.Conv_VectorToRotator` (`KismetMathLibrary.Vector_Normal2D` (`KismetMathLibrary.Conv_RotatorToVector` (`SceneComponent.K2_GetComponentRotation` _sphere3)))) (2.5 2.5 2.5)) "AlwaysSpawn" "OverrideRootScale" null null))

(fn `UserConstructionScript`
  (`parent.UserConstructionScript`))