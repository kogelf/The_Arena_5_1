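; BP_Damage_Pop_UP is an actor that shows a floating damage number and removes itself afterwards.
; On BeginPlay it passes its DamageAmount to the Damage_Pop_UP widget held by its widget component.
; A MovePopup timeline then lerps the actor upward a short distance from its start location and destroys it when finished.
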(event `self.ReceiveBeginPlay`
  (bind _asdamage_pop_up (cast `/Game/Arena_stuff/charecture_folder/universal_hud_folder/Damage_Pop_UP` (`WidgetComponent.GetWidget` (`self.Widget`))))
  (set `/Game/Arena_stuff/charecture_folder/universal_hud_folder/Damage_Pop_UP.Damage Amount` (`self.Damage Amount`) _asdamage_pop_up)
  (bind _output_get (set `self.Start Location` (`self.K2_GetActorLocation`)))
  (set `self.End location` (+ _output_get (0.0 0.0 50.0)))
  (bind (_direction _move_track) (`Timeline|Move popup`)
    (:`Update`
      (`self.K2_SetActorLocation` (`KismetMathLibrary.VLerp` (`self.Start Location`) (`self.End location`) _move_track)))
    (:`Finished`
      (`self.K2_DestroyActor`))))

(fn `UserConstructionScript`)