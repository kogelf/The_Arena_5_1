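; A single-shot crossbow actor that spawns a BP_Bolt projectile from its socket and reloads on BeginPlay or on request.
; Firing spends the ammo, hides the loaded bolt and plays animation and sound; reloading animates, then restores ammo and bolt visibility after a delay.
; TryFire and TryReload wrap these events and always return true, while SwitchMaterial cycles skins.
; Trajectory-prediction debug drawing is present but disconnected.
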(event `self.ReceiveBeginPlay`
  ;[1 1 1] Setup
  (`self.Reload`))

(event `Fire`
  ;[1 1 1] Fire crossbow
  (if (> (`self.Ammo`) 0)
    (`|SpawnActorFromClass` "/Game/LightCrossbow/Blueprints/BP_Bolt.BP_Bolt_C" (`SceneComponent.GetSocketTransform` (`self.Crossbow`) "Bolt" "RTS_World") "Undefined" "OverrideRootScale")
    (`self.SetBoltVisibility` false)
    (`SkeletalMeshComponent.PlayAnimation` (`self.Crossbow`) "/Game/LightCrossbow/Meshes/Crossbow/Anim_Fire.Anim_Fire" false)
    (`/Engine/EditorBlueprintResources/StandardMacros.DecrementInt` (`self.Ammo`)
      (:`  `
        (`GameplayStatics.PlaySoundAtLocation` "/Game/LightCrossbow/Sounds/S_Ballista_Fire.S_Ballista_Fire" (`self.K2_GetActorLocation`)) ; Play firing sound
      ))))

(event `Reload`
  ;[1 1 1] Reload
  (`SkeletalMeshComponent.PlayAnimation` (`self.Crossbow`) "/Game/LightCrossbow/Meshes/Crossbow/Anim_Reload.Anim_Reload" false)
  (`KismetSystemLibrary.Delay` 1.0)
  (set `self.Ammo` 1)
  (`SceneComponent.SetVisibility` (`self.Bolt`) true false))

(event `self.ReceiveTick`
  (params (DeltaSeconds :type "Float (single-precision)")))

(fn `SetBoltVisibility`
  (params (Visible :type Boolean))
  ;[1 1 1] Show or hide the bolt
  (`SceneComponent.SetVisibility` (`self.Bolt`) Visible false))

(fn `SwitchMaterial`
  ;[1 1 1] Switch Material
  (`/Engine/EditorBlueprintResources/StandardMacros.IncrementInt` (`self.MatIdx`)
    (:`  `
      (if (>= (`self.MatIdx`) (`KismetArrayLibrary.Array_Length` (`self.MaterialVariations`)))
        (set `self.MatIdx` 0))
      (`PrimitiveComponent.SetMaterial` (`self.Crossbow`) 0 (`KismetArrayLibrary.Array_Get` (`self.MaterialVariations`) (`self.MatIdx`))))))

(fn `TryFire`
  (returns (Success :type Boolean))
  ;[1 1 1] Fire crossbow
  (`self.Fire`)
  (return true))

(fn `TryReload`
  (returns (Success :type Boolean))
  ;[1 1 1] Start reload
  (`self.Reload`)
  (return true))

(fn `UserConstructionScript`)